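; PathBlock is a block in a chained path that spawns a teleport pad at its Cube's location.
; OnSpawn creates the TeleportPad with a reference back to the block, copies the block's tags onto it and stores it.
; OnHit calls OnSpawn on NextPathBlock, so each hit makes the next block in the chain spawn its pad.
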(event Custom|OnSpawn
  (bind _self self)
  (bind _returnvalue (Game|SpawnActorfromClass "/Game/Blueprints/TeleportPad.TeleportPad_C" (Math|Conversions|ToTransform(Vector) (.Location (Math|Transform|BreakTransform (Transformation|GetWorldTransform (Variables|Default|GetCube _self))))) "AdjustIfPossibleButAlwaysSpawn" 0 _self 0))
  (Variables|/Script/Engine.Actor|SetTags _returnvalue (Variables|Actor|GetTags))
  (Variables|Default|SetTeleportPad _returnvalue))

(event Custom|OnHit
  (CallFunction|OnSpawn (Variables|Default|GetNextPathBlock)))

(fn ConstructionScript)
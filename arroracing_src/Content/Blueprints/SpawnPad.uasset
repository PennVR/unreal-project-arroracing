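; SpawnPad is a pad Blueprint that colors its mesh according to owning player and pad type.
; On BeginPlay it reads the player0 or player1 tag, plus an optional Checkpoint tag, to choose the matching checkpoint or pad material.
; It creates a dynamic instance of that material, stores it as PadMaterial and applies it to the static mesh's first slot.
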(event EventBeginPlay
  (bind _tags (Variables|Actor|GetTags))
  (bind _returnvalue (Utilities|Array|ContainsItem _tags "Checkpoint"))
  ;[1 1 1] Set the pad to an appropriate color
  (if (Utilities|Array|ContainsItem _tags "player0")
    (if _returnvalue
      (bind _returnvalue_2 (Rendering|Material|CreateDynamicMaterialInstance "/Game/FirstPerson/Meshes/CheckpointPlayerOne.CheckpointPlayerOne" :!class /Script/Engine.KismetMaterialLibrary))
      (Variables|Default|SetPadMaterial _returnvalue_2)
      (else
        (bind _returnvalue_3 (Rendering|Material|CreateDynamicMaterialInstance "/Game/FirstPerson/Meshes/PadPlayerOne.PadPlayerOne" :!class /Script/Engine.KismetMaterialLibrary))
        (Variables|Default|SetPadMaterial _returnvalue_3)))
    (Rendering|Material|SetMaterial (Variables|Default|GetStaticMesh) 0 (Variables|Default|GetPadMaterial) :!label _label)
    (elif (Utilities|Array|ContainsItem _tags "player1")
      (if _returnvalue
        (bind _returnvalue_4 (Rendering|Material|CreateDynamicMaterialInstance "/Game/FirstPerson/Meshes/CheckpointPlayerTwo.CheckpointPlayerTwo" :!class /Script/Engine.KismetMaterialLibrary))
        (Variables|Default|SetPadMaterial _returnvalue_4)
        (goto _label)
        (else
          (bind _returnvalue_5 (Rendering|Material|CreateDynamicMaterialInstance "/Game/FirstPerson/Meshes/PadPlayerTwo.PadPlayerTwo" :!class /Script/Engine.KismetMaterialLibrary))
          (Variables|Default|SetPadMaterial _returnvalue_5)
          (goto _label))))))

(fn ConstructionScript)
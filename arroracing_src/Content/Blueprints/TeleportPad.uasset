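; TeleportPad is a moving pad actor that animates around its starting location, with no teleport logic in this graph.
; On BeginPlay it stores that location, seeks Timeline_0 to a random time so its motion starts at a random phase, then plays it.
; Timeline updates add the YPos track to the original location without sweeping.
; ResumePad and PausePad events play and stop the timeline.
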(event Custom|ResumePad
  ;[1 1 1] Spawn randomly-moving teleport pad
  (bind _y_pos (Timeline|Timeline_0 Play)
    (:Update
      (Transformation|SetActorRelativeLocation (+ (Variables|Default|GetOriginal%20Location) _y_pos)))))

(event Custom|PausePad
  ;[1 1 1] Spawn randomly-moving teleport pad
  (bind _y_pos (Timeline|Timeline_0 Stop)
    (:Update
      (Transformation|SetActorRelativeLocation (+ (Variables|Default|GetOriginal%20Location) _y_pos)))))

(event EventBeginPlay
  ;[1 1 1] Spawn randomly-moving teleport pad
  (Variables|Default|SetOriginal%20Location (Transformation|GetActorLocation))
  (Variables|Default|SetOffset (* 8 (Math|Random|RandomFloat)))
  (Utilities|FlowControl|Sequence
    (:then_0
      (bind _y_pos (Timeline|Timeline_0 SetNewTime)
        (:Update
          (Transformation|SetActorRelativeLocation (+ (Variables|Default|GetOriginal%20Location) _y_pos)))))
    (:then_1
      (Timeline|Timeline_0 Play))))

(fn ConstructionScript)